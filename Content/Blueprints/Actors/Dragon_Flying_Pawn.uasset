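; Player-controlled dragon pawn that switches between walking and flying, with Thrust triggering takeoff or a timed boost and SwitchMode setting a braking flag.
; Input axes set walk speed and heading on the ground, or pitch, roll and yaw in the air.
; Tick moves it by swept offsets without a movement component, using CalculateCurrentSpeed for flight speed.
; Hits land it on perfectly flat surfaces or gradually deflect it along other surface normals.
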(event Collision|EventHit
  (params (MyComp :type Primitive%20Component%20Object%20Reference) (Other :type Actor%20Object%20Reference) (OtherComp :type Primitive%20Component%20Object%20Reference) (bSelfMoved :type Boolean) (HitLocation :type Vector :default "0, 0, 0") (HitNormal :type Vector :default "0, 0, 0") (NormalImpulse :type Vector :default "0, 0, 0") (Hit :type Hit%20Result%20Structure%20%28by%20ref%29))
  (bind _returnvalue (Transformation|GetActorRotation))
  (bind _yaw (Math|Rotator|BreakRotator _returnvalue))
  (if (Variables|Default|GetisFlying)
    (if (== (.Z (Math|Vector|BreakVector HitNormal)) 1.0)
      (Variables|Default|SetisFlying false)
      (Transformation|SetActorRotation (Math|Rotator|MakeRotator 0.0 0.0 _yaw) true)
      (Variables|Default|SetCurrentYaw _yaw)
      (Variables|Default|SetCurrentPitch 0.0)
      (Variables|Default|SetCurrentRoll 0.0)
      (else
        ;[1 1 1] Deflect when colliding
        (Transformation|SetActorRotation (Math|Rotator|Lerp(Rotator) (Transformation|GetActorRotation) (Math|Conversions|RotationFromXVector HitNormal) 0.025 true))))
    (elif (== (.Z (Math|Vector|BreakVector HitNormal)) 1.0)
      (Transformation|AddActorLocalOffset (Math|Vector|MakeVector (* (Utilities|Time|GetWorldDeltaSeconds) (Variables|Default|GetCurrentSpeed)) 0.0 0.0) true false))))

(event EventTick
  (params (DeltaSeconds :type Float%20%28single-precision%29))
  (Development|PrintString "" true true "(R=0.000000,G=0.660000,B=1.000000,A=1.000000)" 1e-06)
  (if (Variables|Default|GetisFlying)
    (if (Variables|Default|GetisTakeoff)
      (Transformation|AddActorLocalOffset (Math|Vector|MakeVector 0.0 0.0 (* DeltaSeconds (Variables|Default|GetTakeoffHeight))) true false) ; Lift off the ground
      (else
        ;[1 1 1] Flying movement
        (bind _output_get (Variables|Default|SetCurrentSpeed (|CalculateCurrentSpeed DeltaSeconds)))
        (if (<= _output_get 0.0)
          (Variables|Default|SetCurrentPitch (Math|Interpolation|FInterpTo (Variables|Default|GetCurrentPitch) -5.0 DeltaSeconds 3.0)))
        (Transformation|AddActorLocalOffset (Math|Vector|MakeVector (* _output_get DeltaSeconds) 0.0 0.0) true false)
        (Class|Actor|AddActorWorldRotation (Math|Rotator|MakeRotator 0.0 0.0 (Variables|Default|GetCurrentYaw)))
        (Transformation|SetActorRotation (Math|Rotator|MakeRotator (Variables|Default|GetCurrentRoll) (Variables|Default|GetCurrentPitch) (|GetActorYaw)))))
    (else
      (Transformation|AddActorLocalOffset (Math|Vector|MakeVector (* DeltaSeconds (Variables|Default|GetCurrentSpeed)) 0.0 -9.8) true false)
      (Transformation|SetActorRotation (Math|Rotator|MakeRotator 0.0 0.0 (Variables|Default|GetCurrentYaw))))))

(event Input|ActionEvents|InputActionThrust
  (params (Key :type Key%20Structure))
  (:Pressed
    (if (Variables|Default|GetisFlying)
      ;[1 1 1] Boost
      (Variables|Default|SetCurrentSpeed (Math|Float|Clamp(Float) (+ (Variables|Default|GetCurrentSpeed) (Variables|Default|GetThrustPower)) (Variables|Default|GetSpeedMinFly) (Variables|Default|GetSpeedMaxFly)))
      (Variables|Default|SetisBoosting true)
      (Utilities|FlowControl|Delay 0.7)
      (Variables|Default|SetisBoosting false)
      (else
        ;[1 1 1] Takeoff
        (Variables|Default|SetCurrentYaw 0.0)
        (Variables|Default|SetisFlying true)
        (Variables|Default|SetisTakeoff true)
        (Utilities|FlowControl|Delay (Variables|Default|GetTakeoffTime))
        (Variables|Default|SetisTakeoff false)
        (Variables|Default|SetCurrentPitch 0.0)
        (Variables|Default|SetCurrentRoll 0.0)))))

(event Input|ActionEvents|InputActionSwitchMode
  (params (Key :type Key%20Structure))
  (:Pressed
    (Variables|Default|SetIsBraking true))
  (:Released
    (Variables|Default|SetIsBraking false)))

(event Input|AxisEvents|InputAxisMoveUp
  (params (AxisValue :type Float%20%28single-precision%29))
  (bind _maxpitch (Variables|Default|GetMaxPitch))
  (bind _speedmaxwalk (Variables|Default|GetSpeedMaxWalk))
  (if (Variables|Default|GetisFlying)
    ;[1 1 1] Set pitch
    (Variables|Default|SetCurrentPitch (Math|Float|Clamp(Float) (+ (* AxisValue (Variables|Default|GetSpeedPitch)) (Variables|Default|GetCurrentPitch)) (* -1 _maxpitch) _maxpitch))
    (else
      ;[1 1 1] Set walk speed
      (Variables|Default|SetCurrentSpeed (Math|Float|Clamp(Float) (* AxisValue _speedmaxwalk) (* _speedmaxwalk -0.5) _speedmaxwalk)))))

(event Input|AxisEvents|InputAxisMoveRight
  (params (AxisValue :type Float%20%28single-precision%29))
  (if (Variables|Default|GetisFlying)
    ;[1 1 1] Set roll
    (Variables|Default|SetCurrentRoll (Math|Interpolation|FInterpTo (Variables|Default|GetCurrentRoll) (* AxisValue (Variables|Default|GetMaxRoll)) (Utilities|Time|GetWorldDeltaSeconds) (Variables|Default|GetSpeedRoll)))
    ;[1 1 1] Set yaw
    (Variables|Default|SetCurrentYaw (Math|Interpolation|FInterpTo (Variables|Default|GetCurrentYaw) (* AxisValue (Variables|Default|GetSpeedYaw)) (Utilities|Time|GetWorldDeltaSeconds) 2.0))
    (else
      ;[1 1 1] Set walk angle
      (Variables|Default|SetCurrentYaw (+ (* AxisValue (Variables|Default|GetSpeedYawWalk)) (Variables|Default|GetCurrentYaw))))))

(fn ConstructionScript)
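; Player-controlled dragon character that walks, takes off and flies with momentum-based gliding.
; Input sets speed, pitch, roll and yaw, which Tick applies through manual swept offsets and rotation, switching Walking to Flying when falling.
; In flight, diving gains speed and climbing loses it, with thrust boosts and a brake that also freezes steering.
; Hits on walkable surfaces land the dragon, while other hits nudge its rotation toward the surface normal.
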(event Collision|EventHit
  (params (MyComp :type Primitive%20Component%20Object%20Reference) (Other :type Actor%20Object%20Reference) (OtherComp :type Primitive%20Component%20Object%20Reference) (bSelfMoved :type Boolean) (HitLocation :type Vector :default "0, 0, 0") (HitNormal :type Vector :default "0, 0, 0") (NormalImpulse :type Vector :default "0, 0, 0") (Hit :type Hit%20Result%20Structure%20%28by%20ref%29))
  (bind _returnvalue (Transformation|GetActorRotation))
  (bind _yaw (Math|Rotator|BreakRotator _returnvalue))
  (if (Class|NavMovementComponent|IsFlying (Pawn|GetMovementComponent))
    (if (>= (.Z (Math|Vector|BreakVector HitNormal)) (Class|CharacterMovementComponent|GetWalkableFloorZ (Variables|Character|GetCharacterMovement)))
      (Pawn|Components|CharacterMovement|SetMovementMode (Variables|Character|GetCharacterMovement) "MOVE_Walking" 0)
      (Transformation|SetActorRotation (Math|Rotator|MakeRotator 0.0 0.0 _yaw) true)
      (Variables|Default|SetCurrentYaw _yaw)
      (Variables|Default|SetCurrentPitch 0.0)
      (Variables|Default|SetCurrentRoll 0.0)
      (else
        ;[1 1 1] Deflect when colliding
        (Transformation|SetActorRotation (Math|Rotator|Lerp(Rotator) (Transformation|GetActorRotation) (Math|Conversions|RotationFromXVector HitNormal) 0.025 true))))))

(event Collision|EventActorBeginOverlap
  (params (OtherActor :type Actor%20Object%20Reference)))

(event EventTick
  (params (DeltaSeconds :type Float%20%28single-precision%29))
  (Development|PrintString (Utilities|String|ToString(Float) (Variables|Default|GetCurrentSpeed)) true true "(R=0.000000,G=0.660000,B=1.000000,A=1.000000)" 1e-06)
  (if (Class|NavMovementComponent|IsFlying (Pawn|GetMovementComponent))
    (if (Variables|Default|GetisTakeoff)
      ;[1 1 1] Takeoff
      (Transformation|AddActorLocalOffset (Math|Vector|MakeVector 0.0 0.0 (* DeltaSeconds (Variables|Default|GetTakeoffHeight))) true false) ; Lift off the ground
      (else
        ;[1 1 1] Flying movement
        (if (Variables|Default|GetisBraking)
          ;[1 1 1] Apply Brakes
          (bind _output_get (Variables|Default|SetCurrentSpeed (Math|Float|Clamp(Float) (- (Variables|Default|GetCurrentSpeed) (Variables|Default|GetBrakePower)) 0.0 (Class|MovementComponent|GetMaxSpeed (Variables|Character|GetCharacterMovement)))))
          (Transformation|AddActorLocalOffset (Math|Vector|MakeVector (* _output_get DeltaSeconds) 0.0 0.0) true false)
          (else
            (bind _output_get_2 (Variables|Default|SetCurrentSpeed (|CalculateCurrentSpeed DeltaSeconds)))
            (if (<= _output_get_2 0.0)
              (Variables|Default|SetCurrentPitch (Math|Interpolation|FInterpTo (Variables|Default|GetCurrentPitch) -5.0 DeltaSeconds 3.0)))
            (Transformation|AddActorLocalOffset (Math|Vector|MakeVector (* _output_get_2 DeltaSeconds) 0.0 0.0) true false)
            (Transformation|SetActorRotation (|CalculateAngle))))))
    (else
      ;[1 1 1] Walking
      (Variables|Default|SetLastYaw (Variables|Default|GetCurrentYaw))
      (Transformation|AddActorLocalOffset (Math|Vector|MakeVector (* DeltaSeconds (Variables|Default|GetCurrentSpeed)) 0.0 0.0) true false)
      (Transformation|SetActorRotation (Math|Rotator|MakeRotator 0.0 0.0 (Variables|Default|GetCurrentYaw)))
      ;[1 1 1] Falling to Flying
      (if (AI|Components|NavMovement|IsFalling (Variables|Character|GetCharacterMovement))
        (Variables|Default|SetCurrentYaw 0.0)
        (Pawn|Components|CharacterMovement|SetMovementMode (Variables|Character|GetCharacterMovement) "MOVE_Flying" 0)))))

(event EventBeginPlay)

(event Input|ActionEvents|InputActionThrust
  (params (Key :type Key%20Structure :default "None"))
  (bind _charactermovement (Variables|Character|GetCharacterMovement))
  (:Pressed
    (if (Class|NavMovementComponent|IsFlying (Pawn|GetMovementComponent))
      ;[1 1 1] Boost
      (Variables|Default|SetCurrentSpeed (Math|Float|Clamp(Float) (+ (Variables|Default|GetCurrentSpeed) (Variables|Default|GetThrustPower)) 0.0 (Variables|/Script/Engine.CharacterMovementComponent|GetMaxFlySpeed (Variables|Character|GetCharacterMovement))) :!label _label)
      (Variables|Default|SetisBoosting true)
      (Utilities|FlowControl|Delay 0.7)
      (Variables|Default|SetisBoosting false)
      (else
        ;[1 1 1] Takeoff
        (Variables|Default|SetCurrentYaw 0.0)
        (Pawn|Components|CharacterMovement|SetMovementMode _charactermovement "MOVE_Flying" 0)
        (if (< (Variables|Default|GetCurrentSpeed) (* (Variables|/Script/Engine.CharacterMovementComponent|GetMaxWalkSpeed _charactermovement) 0.75))
          (Variables|Default|SetisTakeoff true)
          (Utilities|FlowControl|Delay (Variables|Default|GetTakeoffTime))
          (Variables|Default|SetisTakeoff false)
          (Variables|Default|SetCurrentPitch 0.0)
          (Variables|Default|SetCurrentRoll 0.0)
          (else
            (Variables|Default|SetCurrentPitch 5e+01)
            (Variables|Default|SetCurrentRoll 0.0)
            (goto _label)))))))

(event Input|ActionEvents|InputActionSwitchMode
  (params (Key :type Key%20Structure :default "None"))
  (:Pressed
    (Variables|Default|SetIsBraking true))
  (:Released
    (Variables|Default|SetIsBraking false)))

(event Input|AxisEvents|InputAxisMoveUp
  (params (AxisValue :type Float%20%28single-precision%29))
  (bind _returnvalue (Pawn|GetMovementComponent))
  (bind _maxpitch (Variables|Default|GetMaxPitch))
  (bind _returnvalue_2 (Class|MovementComponent|GetMaxSpeed _returnvalue))
  (if (Class|NavMovementComponent|IsFlying _returnvalue)
    ;[1 1 1] Set pitch
    (Variables|Default|SetCurrentPitch (Math|Float|Clamp(Float) (+ (* AxisValue (Variables|Default|GetSpeedPitch)) (Variables|Default|GetCurrentPitch)) (* -1 _maxpitch) _maxpitch))
    (else
      ;[1 1 1] Set walk speed
      (Variables|Default|SetCurrentSpeed (Math|Float|Clamp(Float) (* AxisValue _returnvalue_2) (* _returnvalue_2 -0.5) _returnvalue_2)))))

(event Input|AxisEvents|InputAxisMoveRight
  (params (AxisValue :type Float%20%28single-precision%29))
  (if (Class|NavMovementComponent|IsFlying (Pawn|GetMovementComponent))
    ;[1 1 1] Set roll
    (Variables|Default|SetCurrentRoll (Math|Interpolation|FInterpTo (Variables|Default|GetCurrentRoll) (* AxisValue (Variables|Default|GetMaxRoll)) (Utilities|Time|GetWorldDeltaSeconds) (Variables|Default|GetSpeedRoll)))
    ;[1 1 1] Set yaw
    (Variables|Default|SetCurrentYaw (Math|Interpolation|FInterpTo (Variables|Default|GetCurrentYaw) (* AxisValue (Variables|Default|GetSpeedYaw)) (Utilities|Time|GetWorldDeltaSeconds) 2.0))
    (else
      ;[1 1 1] Set walk angle
      (Variables|Default|SetCurrentYaw (+ (* AxisValue (Variables|Default|GetSpeedYawWalk)) (Variables|Default|GetCurrentYaw))))))

(fn ConstructionScript
  (Pawn|Components|CharacterMovement|SetMovementMode (Variables|Character|GetCharacterMovement) "MOVE_Walking" 0))